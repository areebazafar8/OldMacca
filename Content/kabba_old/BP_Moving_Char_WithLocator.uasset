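; A character Blueprint that drives an on-screen compass pointing toward a North_Marker actor in the level.
; On BeginPlay it creates the Compass_Widget, adds it to the viewport and caches the marker's location.
; Each Tick it rotates the compass pointer by the look-at yaw from the character to the marker minus the control rotation yaw, keeping it relative to the view.
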(event EventBeginPlay
  (bind _returnvalue (UserInterface|CreateWidget "/Game/kabba_old/Compass_Widget.Compass_Widget_C"))
  (bind _output_get (Variables|Default|SetCompass_Ref _returnvalue))
  (UserInterface|Viewport|AddtoViewport _output_get 0)
  (bind _returnvalue_2 (Actor|GetActorOfClass "/Game/kabba_old/North_Marker.North_Marker_C"))
  (Variables|Default|SetNorth_Location (Transformation|GetActorLocation _returnvalue_2)))

(event EventTick
  (params (DeltaSeconds :type Float%20%28single-precision%29))
  (Class|Widget|SetRenderTransformAngle (Variables|/Game/kabba_old/Compass_Widget.Compass_Widget_C|GetCompassPointer (Variables|Default|GetCompass_Ref)) (- (.yaw (Math|Rotator|FindLookatRotation (Transformation|GetActorLocation) (Variables|Default|GetNorth_Location))) (.yaw (Pawn|GetControlRotation :!class /Script/Engine.Pawn)))))

(fn ConstructionScript)